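; Blueprint function library with shared helpers for player access and pick-actor proximity lookup.
; GetBpPlayerRef returns the pawn of player index 0 cast to BP_Player.
; GetNearestPickActor loops over a given actor list, tracking a running minimum distance to a reference actor, and returns the nearest match.
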(fn `GetBpPlayerRef`
  (returns (Value :type "/Game/MyContent/BluePrints/PlayerGame/BP_Player Object Reference"))
  (bind _asbp_player (cast `/Game/MyContent/BluePrints/PlayerGame/BP_Player` (`GameplayStatics.GetPlayerPawn` null)))
  (return _asbp_player))

(fn `GetNearestPickActor`
  (params (PickActorList :type "Array of Actor Object Reference") (Actor :type "Actor Object Reference"))
  (returns (ReturnValue :type "Actor Object Reference"))
  (locals (distance :type "Float (double-precision)" :default 500.0) (nearestActor :type "Actor Object Reference"))
  (for _array_element PickActorList
    (bind _returnvalue (`Actor.GetDistanceTo` _array_element Actor))
    (if (< _returnvalue (`local.distance`))
      (set `local.distance` _returnvalue)
      (set `local.nearestActor` _array_element)))
  (return (`local.nearestActor`)))