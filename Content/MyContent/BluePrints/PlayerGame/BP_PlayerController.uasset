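; Player controller Blueprint that turns player input into movement, camera and action commands for the controlled character.
; Move axes add movement input to the controlled pawn along the controller's own forward and right vectors, while look axes drive pitch and yaw.
; Jump and PickUp presses call events on the player Blueprint reference, with a validity check only on PickUp.
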(event `InputAxis|MoveForward`
  (params (AxisValue :type "Float (single-precision)"))
  (`Pawn.AddMovementInput` (`self.K2_GetPawn`) (`self.GetActorForwardVector`) AxisValue false))

(event `InputAxis|MoveRight`
  (params (AxisValue :type "Float (single-precision)"))
  (`Pawn.AddMovementInput` (`self.K2_GetPawn`) (`self.GetActorRightVector`) AxisValue false))

(event `InputAxis|LookUp`
  (params (AxisValue :type "Float (single-precision)"))
  (`self.AddPitchInput` AxisValue))

(event `InputAxis|LookTurn`
  (params (AxisValue :type "Float (single-precision)"))
  (`self.AddYawInput` AxisValue))

(event `InputAction|Jump`
  (params (Key :type "Key Structure"))
  (:`Pressed`
    (bind _value (`/Game/MyContent/BluePrints/Library/FunctionLibrary.GetBpPlayerRef`))
    (`/Game/MyContent/BluePrints/PlayerGame/BP_Player.JumpEvent` _value)))

(event `InputAction|PickUp`
  (params (Key :type "Key Structure"))
  (:`Pressed`
    (bind _value (`/Game/MyContent/BluePrints/Library/FunctionLibrary.GetBpPlayerRef`))
    (`/Engine/EditorBlueprintResources/StandardMacros.IsValid` _value
      (:`Is Valid`
        (`/Game/MyContent/BluePrints/PlayerGame/BP_Player.PickUpEvent` _value)))))

(fn `UserConstructionScript`)