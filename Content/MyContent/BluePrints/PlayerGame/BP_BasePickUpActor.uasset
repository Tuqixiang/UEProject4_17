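; BP_BasePickUpActor is a base pickup actor that registers itself with the player while in range.
; On capsule begin overlap with BP_Player, it adds itself to PickUpActorArray and creates a tip panel through MainUI from its texture and text.
; End overlap removes it from that array and removes the stored panel from its parent.
; The BePickUp event only destroys the actor.
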(event `self.Capsule.OnComponentBeginOverlap`
  (params (OverlappedComponent :type "PrimitiveComponent Object Reference") (OtherActor :type "Actor Object Reference") (OtherComp :type "PrimitiveComponent Object Reference") (OtherBodyIndex :type Integer) (bFromSweep :type Boolean) (SweepResult :type "HitResult Structure (by ref)"))
  (bind _asbp_player (cast `/Game/MyContent/BluePrints/PlayerGame/BP_Player` OtherActor))
  (`KismetArrayLibrary.Array_AddUnique` (`/Game/MyContent/BluePrints/PlayerGame/BP_Player.PickUpActorArray` _asbp_player) self)
  (bind _returnvalue (`/Game/MyContent/BluePrints/UI/WB_MainPanel.TipFunction` (`/Game/MyContent/BluePrints/PlayerGame/BP_Player.MainUI` _asbp_player) (`self.TP_Texture`) (`self.TP_TipText`)))
  (set `self.tipPanelRef` _returnvalue))

(event `self.Capsule.OnComponentEndOverlap`
  (params (OverlappedComponent :type "PrimitiveComponent Object Reference") (OtherActor :type "Actor Object Reference") (OtherComp :type "PrimitiveComponent Object Reference") (OtherBodyIndex :type Integer))
  (bind _asbp_player (cast `/Game/MyContent/BluePrints/PlayerGame/BP_Player` OtherActor))
  (`KismetArrayLibrary.Array_RemoveItem` (`/Game/MyContent/BluePrints/PlayerGame/BP_Player.PickUpActorArray` _asbp_player) self)
  (`Widget.RemoveFromParent` (`self.tipPanelRef`)))

(event `BePickUp`
  (`self.K2_DestroyActor`))

(fn `UserConstructionScript`)